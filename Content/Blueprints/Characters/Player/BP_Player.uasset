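; Player character Blueprint that uses the Gameplay Ability System for health regen, dash and laser abilities.
; On BeginPlay it grants the abilities, registers them in the controller's UI and binds attribute changes to the health, mana and strength balls; death disables input.
; Capsule overlaps with actors of another class send a dash damage gameplay event, once per recorded actor.
; Helper functions switch between camera-locked and movement-oriented rotation.
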(event `self.OnHealthChange`
  (params (CurrentValue :type "Float (single-precision)") (MaxValue :type "Float (single-precision)"))
  (`parent.OnHealthChange` CurrentValue MaxValue)
  (`/Game/Blueprints/Widget/WBP_GlassBall.SetPercentage` (`/Game/Blueprints/Widget/WBP_MainUI.HealthBall` (`/Game/Blueprints/Characters/Player/BP_PlayerController.MainUIRef` (`self.ControlRef`))) (/ CurrentValue MaxValue))
  (if (`self.IsDead`)
    (`self.DisableInput` (`self.ControlRef`) null)))

(event `self.ReceiveBeginPlay`
  (bind _attributeset (`self.AttributeSet`))
  (`parent.ReceiveBeginPlay`)
  (`|ExecutionSequence`
    (:`then_0`
      (bind _asbp_player_controller (cast `/Game/Blueprints/Characters/Player/BP_PlayerController` (`self.GetController`)))
      (set `self.ControlRef` _asbp_player_controller))
    (:`then_1`
      (`|ExecutionSequence`
        (:`then_0`
          (bind _returnvalue (`self.AquireAbility` "/Game/Blueprints/Gameplay/Abilities/HealthRegen/GAB_HealthRegen.GAB_HealthRegen_C"))
          (`/Game/Blueprints/Characters/Player/BP_PlayerController.AddAbilityToUI` (`self.ControlRef`) _returnvalue 0))
        (:`then_1`
          (bind _returnvalue_2 (`self.AquireAbility` "/Game/Blueprints/Gameplay/Abilities/Dash/GAB_Dash.GAB_Dash_C"))
          (`/Game/Blueprints/Characters/Player/BP_PlayerController.AddAbilityToUI` (`self.ControlRef`) _returnvalue_2 1))
        (:`then_2`
          (bind _returnvalue_3 (`self.AquireAbility` "/Game/Blueprints/Gameplay/Abilities/Laser/GAB_Laser.GAB_Laser_C"))
          (`/Game/Blueprints/Characters/Player/BP_PlayerController.AddAbilityToUI` (`self.ControlRef`) _returnvalue_3 2))))
    (:`then_2`
      (add `BaseAttributeSet.OnManaChange` _attributeset (delegate `OnManaChange`)))
    (:`then_3`
      (add `BaseAttributeSet.OnStrengthChange` _attributeset (delegate `OnStrengthChange`)))))

(event `OnManaChange`
  (params (CurrentValue :type "Float (double-precision)") (MaxValue :type "Float (double-precision)"))
  (`/Game/Blueprints/Widget/WBP_GlassBall.SetPercentage` (`/Game/Blueprints/Widget/WBP_MainUI.ManaBall` (`/Game/Blueprints/Characters/Player/BP_PlayerController.MainUIRef` (`self.ControlRef`))) (/ CurrentValue MaxValue)))

(event `OnStrengthChange`
  (params (CurrentValue :type "Float (double-precision)") (MaxValue :type "Float (double-precision)"))
  (`/Game/Blueprints/Widget/WBP_GlassBall.SetPercentage` (`/Game/Blueprints/Widget/WBP_MainUI.StrengthBall` (`/Game/Blueprints/Characters/Player/BP_PlayerController.MainUIRef` (`self.ControlRef`))) (/ CurrentValue MaxValue)))

(event `HealthRegeon`
  (`AbilitySystemComponent.TryActivateAbilityByClass` (`self.AbilitySystemComponent`) "/Game/Blueprints/Gameplay/Abilities/HealthRegen/GAB_HealthRegen.GAB_HealthRegen_C" true))

(event `Laser`
  (`AbilitySystemComponent.TryActivateAbilityByClass` (`self.AbilitySystemComponent`) "/Game/Blueprints/Gameplay/Abilities/Laser/GAB_Laser.GAB_Laser_C" true))

(event `Dash`
  (`AbilitySystemComponent.TryActivateAbilityByClass` (`self.AbilitySystemComponent`) "/Game/Blueprints/Gameplay/Abilities/Dash/GAB_Dash.GAB_Dash_C" true))

(event `self.CapsuleComponent.OnComponentBeginOverlap`
  (params (OverlappedComponent :type "PrimitiveComponent Object Reference") (OtherActor :type "Actor Object Reference") (OtherComp :type "PrimitiveComponent Object Reference") (OtherBodyIndex :type Integer) (bFromSweep :type Boolean) (SweepResult :type "HitResult Structure (by ref)"))
  (bind _overlappedenemies (`self.OverlappedEnemies`))
  (if (!= (`GameplayStatics.GetObjectClass` OtherActor) (`GameplayStatics.GetObjectClass` self))
    (if (not (`KismetArrayLibrary.Array_Contains` _overlappedenemies OtherActor))
      (`KismetArrayLibrary.Array_AddUnique` _overlappedenemies OtherActor)
      (`AbilitySystemBlueprintLibrary.SendGameplayEventToActor` self (struct :`TagName` "Ability.Dash.Damage.Event") (make `GameplayEventData` (struct) self OtherActor)))))

(fn `FreeCameraOrientation`
  (`|ExecutionSequence`
    (:`then_0`
      (set `self.bUseControllerRotationYaw` false))
    (:`then_1`
      (set `CharacterMovementComponent.bOrientRotationToMovement` true (`self.CharacterMovement`)))))

(fn `LockCameraOrientation`
  (`|ExecutionSequence`
    (:`then_0`
      (set `self.bUseControllerRotationYaw` true))
    (:`then_1`
      (set `CharacterMovementComponent.bOrientRotationToMovement` false (`self.CharacterMovement`)))))

(fn `UserConstructionScript`
  (`parent.UserConstructionScript`))