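; Player controller that turns input into movement, camera control and ability calls on the possessed BP_Player.
; Number keys trigger regen, dash, laser toggle, ground blast and fire blast, gated by laser and targeting flags.
; Mouse buttons confirm or cancel Ability System targeting, with left click meleeing when not targeting; look-up pitch is clamped.
; BeginPlay caches the pawn and creates the main UI, whose ability slots AddAbilityToUI fills.
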(event `Key|One`
  (params (Key :type "Key Structure"))
  (:`Pressed`
    (`/Game/Blueprints/Characters/Player/BP_Player.HealthRegeon` (`self.PlayerRef`))))

(event `Key|Two`
  (params (Key :type "Key Structure"))
  (:`Pressed`
    (`/Game/Blueprints/Characters/Player/BP_Player.Dash` (`self.PlayerRef`))))

(event `Key|Three`
  (params (Key :type "Key Structure"))
  (bind _playerref (`self.PlayerRef`))
  (:`Pressed`
    (if (`self.DoingLaser`)
      (`/Game/Blueprints/Characters/Player/BP_Player.CancelLaser` _playerref)
      (else
        (`/Game/Blueprints/Characters/Player/BP_Player.Laser` _playerref)))))

(event `Key|Four`
  (params (Key :type "Key Structure"))
  (:`Pressed`
    (if (not (`self.Targeting`))
      (`/Game/Blueprints/Characters/Player/BP_Player.GroundBlast` (`self.PlayerRef`)))))

(event `InputAxis|MoveForward`
  (params (AxisValue :type "Float (single-precision)"))
  (bind _playerref (`self.PlayerRef`))
  ;[1 1 1] Player
  (`Pawn.AddMovementInput` _playerref (`SceneComponent.GetForwardVector` (`/Game/Blueprints/Characters/Player/BP_Player.Camera` _playerref)) (* AxisValue 100.0) false))

(event `Key|Five`
  (params (Key :type "Key Structure"))
  (:`Pressed`
    (`/Game/Blueprints/Characters/Player/BP_Player.FireBlast` (`self.PlayerRef`))))

(event `InputAxis|MoveRight`
  (params (AxisValue :type "Float (single-precision)"))
  (bind _playerref (`self.PlayerRef`))
  ;[1 1 1] Player
  (`Pawn.AddMovementInput` _playerref (`SceneComponent.GetRightVector` (`/Game/Blueprints/Characters/Player/BP_Player.Camera` _playerref)) (* AxisValue 100.0) false))

(event `self.ReceiveBeginPlay`
  (`|ExecutionSequence`
    (:`then_0`
      ;[1 1 1] Player
      (bind _asbp_player (cast `/Game/Blueprints/Characters/Player/BP_Player` (`self.K2_GetPawn`)))
      (set `self.PlayerRef` _asbp_player))
    (:`then_1`
      (bind _returnvalue (`|CreateWidget` "/Game/Blueprints/Widget/WBP_MainUI.WBP_MainUI_C"))
      (set `self.MainUIRef` _returnvalue)
      (`UserWidget.AddToViewport` _returnvalue 0))))

(event `InputAxis|Turn`
  (params (AxisValue :type "Float (single-precision)"))
  ;[1 1 1] Player
  (`self.AddYawInput` AxisValue))

(event `InputAction|Jump`
  (params (Key :type "Key Structure"))
  ;[1 1 1] Player
  (:`Pressed`
    (`Character.Jump` (`self.PlayerRef`))))

(event `Key|LeftMouseButton`
  (params (Key :type "Key Structure"))
  (:`Pressed`
    (if (`self.Targeting`)
      (`AbilitySystemComponent.TargetConfirm` (`BaseCharacter.AbilitySystemComponent` (`self.PlayerRef`)))
      (set `self.Targeting` false)
      (else
        (`/Game/Blueprints/Characters/Bp_BaseCharacter.MeleeAttack` (`self.PlayerRef`))))))

(event `InputAxis|LookUp`
  (params (AxisValue :type "Float (single-precision)"))
  (bind (_returnvalue_roll _returnvalue_pitch) (`KismetMathLibrary.BreakRotator` (`self.GetControlRotation`)))
  (bind _returnvalue (+ _returnvalue_pitch (* AxisValue (`self.InputPitchScale`))))
  ;[1 1 1] Player
  (if (or (and (> _returnvalue -999.0) (< _returnvalue 45.0)) (and (> _returnvalue 300.0) (<= _returnvalue 999.0)))
    (`self.AddPitchInput` AxisValue)))

(event `Key|RightMouseButton`
  (params (Key :type "Key Structure"))
  (:`Pressed`
    (`AbilitySystemComponent.TargetCancel` (`BaseCharacter.AbilitySystemComponent` (`self.PlayerRef`)))))

(fn `AddAbilityToUI`
  (params (AbilityInfo :type "GameplayAbilityInfo Structure") (AbilityIndex :type Integer))
  (`/Game/Blueprints/Widget/WBP_AbilitySlot.SetSlotInfo` (`|GetArrayItem` (`/Game/Blueprints/Widget/WBP_MainUI.Slots` (`self.MainUIRef`)) AbilityIndex) AbilityInfo (`KismetTextLibrary.Conv_IntToText` (+ AbilityIndex 1))))

(fn `UserConstructionScript`)