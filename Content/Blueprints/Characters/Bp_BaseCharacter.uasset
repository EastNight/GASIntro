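; Base character Blueprint built on the Gameplay Ability System, with a melee attack and death handling.
; On BeginPlay it caches ground friction, binds to attribute-set health changes and grants the melee ability, which MeleeAttack activates.
; Weapon overlaps with actors of a different class send a damage gameplay event to itself, targeting the other actor.
; Zero health plays a death montage, then destroys the actor; helper functions zero or restore ground friction.
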(event `self.ReceiveBeginPlay`
  (`|ExecutionSequence`
    (:`then_0`
      (set `self.DefaultGroundFriction` (`CharacterMovementComponent.GroundFriction` (`self.CharacterMovement`))))
    (:`then_1`
      (add `BaseAttributeSet.OnHealthChange` (`self.AttributeSet`) (delegate `OnHealthChange`)))
    (:`then_2`
      (`self.AquireAbility` "/Game/Blueprints/Gameplay/Abilities/MeleeAttack/GAB_MeleeAttack.GAB_MeleeAttack_C"))))

(event `OnHealthChange`
  (params (CurrentValue :type "Float (double-precision)") (MaxValue :type "Float (double-precision)"))
  (if (and (not (`self.IsDead`)) (<= CurrentValue 0.0))
    (set `self.IsDead` true)
    (bind _returnvalue (`self.PlayAnimMontage` "/Game/Animations/Characters/Montages/AM_Die.AM_Die"))
    (`KismetSystemLibrary.Delay` _returnvalue)
    (`self.K2_DestroyActor`)))

(event `MeleeAttack`
  (`AbilitySystemComponent.TryActivateAbilityByClass` (`self.AbilitySystemComponent`) "/Game/Blueprints/Gameplay/Abilities/MeleeAttack/GAB_MeleeAttack.GAB_MeleeAttack_C" true))

(event `self.WeaponCollision.OnComponentBeginOverlap`
  (params (OverlappedComponent :type "PrimitiveComponent Object Reference") (OtherActor :type "Actor Object Reference") (OtherComp :type "PrimitiveComponent Object Reference") (OtherBodyIndex :type Integer) (bFromSweep :type Boolean) (SweepResult :type "HitResult Structure (by ref)"))
  (if (not (or (== (`GameplayStatics.GetObjectClass` self) (`GameplayStatics.GetObjectClass` OtherActor)) (== OtherActor self)))
    (`AbilitySystemBlueprintLibrary.SendGameplayEventToActor` self (struct :`TagName` "Ability.MeleeAttack.Damage.Event") (make `GameplayEventData` (struct :`TagName` "Ability.MeleeAttack.Damage.Event") null OtherActor))))

(event `self.ReceiveTick`
  (params (DeltaSeconds :type "Float (single-precision)")))

(fn `SetGroundFrictionDefault`
  (set `CharacterMovementComponent.GroundFriction` (`self.DefaultGroundFriction`) (`self.CharacterMovement`)))

(fn `SetGroundFrictionZero`
  (set `CharacterMovementComponent.GroundFriction` 0.0 (`self.CharacterMovement`)))

(fn `UserConstructionScript`)